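; FrostMissile_BP is a frost missile that slows orc characters caught in its SlowDown area.
; Every Tick it cuts the MaxWalkSpeed of each overlapping OrcCharacter to a tenth of its current value and prints its name.
; The slow compounds each frame and is never restored here.
; BeginPlay mutes the Loop sound by setting its volume multiplier to zero.
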(event `self.ReceiveBeginPlay`
  (`AudioComponent.SetVolumeMultiplier` (`self.Loop`) 0.0))

(event `self.ReceiveTick`
  (params (DeltaSeconds :type "Float (single-precision)"))
  (for _array_element (`PrimitiveComponent.GetOverlappingActors` (`self.SlowDown`) "/Script/HobbitMage.OrcCharacter")
    (bind _asorc_character (cast `OrcCharacter` _array_element))
    (bind _charactermovement (`Character.CharacterMovement` _asorc_character))
    (set `CharacterMovementComponent.MaxWalkSpeed` (* (`CharacterMovementComponent.MaxWalkSpeed` _charactermovement) 0.1) _charactermovement)
    (`KismetSystemLibrary.PrintString` (`KismetSystemLibrary.GetDisplayName` _asorc_character))))

(fn `UserConstructionScript`)