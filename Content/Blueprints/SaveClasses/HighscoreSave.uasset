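; HighscoreSave is a save-class Blueprint that holds a Highscore array and can order it from highest to lowest.
; Its Sort function runs an in-place insertion sort, shifting smaller earlier entries up one slot and writing each score into the gap.
; The local named Index holds the score being inserted, while J tracks the array position.
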(fn `Sort`
  (locals (Index :type Integer) (j :type Integer))
  (bind _highscore (`self.Highscore`))
  (for (_array_element _array_index) _highscore
    (bind _output_get (set `local.Index` _array_element))
    (bind _output_get_2 (set `local.j` _array_index))
    (bind _output (`|GetArrayItem` _highscore (- _output_get_2 1)))
    (while (and (> _output_get_2 0) (> _output_get _output))
      (`KismetArrayLibrary.Array_Set` (`self.Highscore`) _output_get_2 _output true)
      (set `local.j` (- (`local.j`) 1)))
    (`KismetArrayLibrary.Array_Set` (`self.Highscore`) (`local.j`) (`local.Index`) true)))