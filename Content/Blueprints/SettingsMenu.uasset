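; In-world settings menu actor that lets the MagePawn adjust quality and other settings through overlap trigger components, registering itself on the pawn at BeginPlay.
; Each trigger acts as a dwell button, calling increase or decrease functions on the pawn's widget after a short delay unless the shared OverlapEnded flag is set.
; Back and Apply also hide the menu widget, disable child overlap events and reveal the root of the "WRE"-tagged actor.
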(event `self.ReceiveBeginPlay`
  (bind _asmage_pawn_bp (cast `/Game/Blueprints/MagePawn_BP` (`GameplayStatics.GetPlayerPawn` 0)))
  (set `/Game/Blueprints/MagePawn_BP.SettingsMenuRef` self _asmage_pawn_bp))

(event `self.ReceiveActorBeginOverlap`
  (params (OtherActor :type "Actor Object Reference")))

(event `self.DD_decC.OnComponentBeginOverlap`
  (params (OverlappedComponent :type "PrimitiveComponent Object Reference") (OtherActor :type "Actor Object Reference") (OtherComp :type "PrimitiveComponent Object Reference") (OtherBodyIndex :type Integer) (bFromSweep :type Boolean) (SweepResult :type "HitResult Structure (by ref)"))
  (bind _asmage_pawn_bp (cast `/Game/Blueprints/MagePawn_BP` OtherActor))
  (set `self.OverlapEnded` false)
  (`KismetSystemLibrary.Delay` 2.0)
  (if (not (`self.OverlapEnded`))
    (`/Game/Blueprints/SettingsWidget.PPAAQ_decrease` (`/Game/Blueprints/MagePawn_BP.WidgetRef` _asmage_pawn_bp))))

(event `self.DD_decC.OnComponentEndOverlap`
  (params (OverlappedComponent :type "PrimitiveComponent Object Reference") (OtherActor :type "Actor Object Reference") (OtherComp :type "PrimitiveComponent Object Reference") (OtherBodyIndex :type Integer))
  (cast `/Game/Blueprints/MagePawn_BP` OtherActor)
  (set `self.OverlapEnded` true))

(event `self.DD_incC.OnComponentBeginOverlap`
  (params (OverlappedComponent :type "PrimitiveComponent Object Reference") (OtherActor :type "Actor Object Reference") (OtherComp :type "PrimitiveComponent Object Reference") (OtherBodyIndex :type Integer) (bFromSweep :type Boolean) (SweepResult :type "HitResult Structure (by ref)"))
  (bind _asmage_pawn_bp (cast `/Game/Blueprints/MagePawn_BP` OtherActor))
  (set `self.OverlapEnded` false)
  (`KismetSystemLibrary.Delay` 2.0)
  (if (not (`self.OverlapEnded`))
    (`/Game/Blueprints/SettingsWidget.PPAAQ_increase` (`/Game/Blueprints/MagePawn_BP.WidgetRef` _asmage_pawn_bp))))

(event `self.DD_incC.OnComponentEndOverlap`
  (params (OverlappedComponent :type "PrimitiveComponent Object Reference") (OtherActor :type "Actor Object Reference") (OtherComp :type "PrimitiveComponent Object Reference") (OtherBodyIndex :type Integer))
  (cast `/Game/Blueprints/MagePawn_BP` OtherActor)
  (set `self.OverlapEnded` true))

(event `self.SQ_decC.OnComponentBeginOverlap`
  (params (OverlappedComponent :type "PrimitiveComponent Object Reference") (OtherActor :type "Actor Object Reference") (OtherComp :type "PrimitiveComponent Object Reference") (OtherBodyIndex :type Integer) (bFromSweep :type Boolean) (SweepResult :type "HitResult Structure (by ref)"))
  (bind _asmage_pawn_bp (cast `/Game/Blueprints/MagePawn_BP` OtherActor))
  (set `self.OverlapEnded` false)
  (`KismetSystemLibrary.Delay` 1.0)
  (if (not (`self.OverlapEnded`))
    (`/Game/Blueprints/SettingsWidget.Q_decrease` (`/Game/Blueprints/MagePawn_BP.WidgetRef` _asmage_pawn_bp) (`self.ShadowQuality`))))

(event `self.SQ_decC.OnComponentEndOverlap`
  (params (OverlappedComponent :type "PrimitiveComponent Object Reference") (OtherActor :type "Actor Object Reference") (OtherComp :type "PrimitiveComponent Object Reference") (OtherBodyIndex :type Integer))
  (cast `/Game/Blueprints/MagePawn_BP` OtherActor)
  (set `self.OverlapEnded` true))

(event `self.SQ_incC.OnComponentBeginOverlap`
  (params (OverlappedComponent :type "PrimitiveComponent Object Reference") (OtherActor :type "Actor Object Reference") (OtherComp :type "PrimitiveComponent Object Reference") (OtherBodyIndex :type Integer) (bFromSweep :type Boolean) (SweepResult :type "HitResult Structure (by ref)"))
  (bind _asmage_pawn_bp (cast `/Game/Blueprints/MagePawn_BP` OtherActor))
  (set `self.OverlapEnded` false)
  (`KismetSystemLibrary.Delay` 1.0)
  (if (not (`self.OverlapEnded`))
    (`/Game/Blueprints/SettingsWidget.Q_Increase` (`/Game/Blueprints/MagePawn_BP.WidgetRef` _asmage_pawn_bp) (`self.ShadowQuality`))))

(event `self.SQ_incC.OnComponentEndOverlap`
  (params (OverlappedComponent :type "PrimitiveComponent Object Reference") (OtherActor :type "Actor Object Reference") (OtherComp :type "PrimitiveComponent Object Reference") (OtherBodyIndex :type Integer))
  (cast `/Game/Blueprints/MagePawn_BP` OtherActor)
  (set `self.OverlapEnded` true))

(event `self.TQ_decC.OnComponentBeginOverlap`
  (params (OverlappedComponent :type "PrimitiveComponent Object Reference") (OtherActor :type "Actor Object Reference") (OtherComp :type "PrimitiveComponent Object Reference") (OtherBodyIndex :type Integer) (bFromSweep :type Boolean) (SweepResult :type "HitResult Structure (by ref)"))
  (bind _asmage_pawn_bp (cast `/Game/Blueprints/MagePawn_BP` OtherActor))
  (set `self.OverlapEnded` false)
  (`KismetSystemLibrary.Delay` 1.0)
  (if (not (`self.OverlapEnded`))
    (`/Game/Blueprints/SettingsWidget.Q_decrease` (`/Game/Blueprints/MagePawn_BP.WidgetRef` _asmage_pawn_bp) (`self.PostProcessQuality`))))

(event `self.TQ_decC.OnComponentEndOverlap`
  (params (OverlappedComponent :type "PrimitiveComponent Object Reference") (OtherActor :type "Actor Object Reference") (OtherComp :type "PrimitiveComponent Object Reference") (OtherBodyIndex :type Integer))
  (cast `/Game/Blueprints/MagePawn_BP` OtherActor)
  (set `self.OverlapEnded` true))

(event `self.TQ_incC.OnComponentBeginOverlap`
  (params (OverlappedComponent :type "PrimitiveComponent Object Reference") (OtherActor :type "Actor Object Reference") (OtherComp :type "PrimitiveComponent Object Reference") (OtherBodyIndex :type Integer) (bFromSweep :type Boolean) (SweepResult :type "HitResult Structure (by ref)"))
  (bind _asmage_pawn_bp (cast `/Game/Blueprints/MagePawn_BP` OtherActor))
  (set `self.OverlapEnded` false)
  (`KismetSystemLibrary.Delay` 1.0)
  (if (not (`self.OverlapEnded`))
    (`/Game/Blueprints/SettingsWidget.Q_Increase` (`/Game/Blueprints/MagePawn_BP.WidgetRef` _asmage_pawn_bp) (`self.PostProcessQuality`))))

(event `self.TQ_incC.OnComponentEndOverlap`
  (params (OverlappedComponent :type "PrimitiveComponent Object Reference") (OtherActor :type "Actor Object Reference") (OtherComp :type "PrimitiveComponent Object Reference") (OtherBodyIndex :type Integer))
  (cast `/Game/Blueprints/MagePawn_BP` OtherActor)
  (set `self.OverlapEnded` true))

(event `self.EQ_decC.OnComponentBeginOverlap`
  (params (OverlappedComponent :type "PrimitiveComponent Object Reference") (OtherActor :type "Actor Object Reference") (OtherComp :type "PrimitiveComponent Object Reference") (OtherBodyIndex :type Integer) (bFromSweep :type Boolean) (SweepResult :type "HitResult Structure (by ref)"))
  (bind _asmage_pawn_bp (cast `/Game/Blueprints/MagePawn_BP` OtherActor))
  (set `self.OverlapEnded` false)
  (`KismetSystemLibrary.Delay` 1.0)
  (if (not (`self.OverlapEnded`))
    (`/Game/Blueprints/SettingsWidget.Q_decrease` (`/Game/Blueprints/MagePawn_BP.WidgetRef` _asmage_pawn_bp) (`self.EffectsQuality`))))

(event `self.EQ_decC.OnComponentEndOverlap`
  (params (OverlappedComponent :type "PrimitiveComponent Object Reference") (OtherActor :type "Actor Object Reference") (OtherComp :type "PrimitiveComponent Object Reference") (OtherBodyIndex :type Integer))
  (cast `/Game/Blueprints/MagePawn_BP` OtherActor)
  (set `self.OverlapEnded` true))

(event `self.EQ_incC.OnComponentBeginOverlap`
  (params (OverlappedComponent :type "PrimitiveComponent Object Reference") (OtherActor :type "Actor Object Reference") (OtherComp :type "PrimitiveComponent Object Reference") (OtherBodyIndex :type Integer) (bFromSweep :type Boolean) (SweepResult :type "HitResult Structure (by ref)"))
  (bind _asmage_pawn_bp (cast `/Game/Blueprints/MagePawn_BP` OtherActor))
  (set `self.OverlapEnded` false)
  (`KismetSystemLibrary.Delay` 1.0)
  (if (not (`self.OverlapEnded`))
    (`/Game/Blueprints/SettingsWidget.Q_Increase` (`/Game/Blueprints/MagePawn_BP.WidgetRef` _asmage_pawn_bp) (`self.EffectsQuality`))))

(event `self.EQ_incC.OnComponentEndOverlap`
  (params (OverlappedComponent :type "PrimitiveComponent Object Reference") (OtherActor :type "Actor Object Reference") (OtherComp :type "PrimitiveComponent Object Reference") (OtherBodyIndex :type Integer))
  (cast `/Game/Blueprints/MagePawn_BP` OtherActor)
  (set `self.OverlapEnded` true))

(event `self.AV_dec.OnComponentBeginOverlap`
  (params (OverlappedComponent :type "PrimitiveComponent Object Reference") (OtherActor :type "Actor Object Reference") (OtherComp :type "PrimitiveComponent Object Reference") (OtherBodyIndex :type Integer) (bFromSweep :type Boolean) (SweepResult :type "HitResult Structure (by ref)"))
  (bind _asmage_pawn_bp (cast `/Game/Blueprints/MagePawn_BP` OtherActor))
  (set `self.OverlapEnded` false)
  (`KismetSystemLibrary.Delay` 1.0)
  (if (not (`self.OverlapEnded`))
    (`/Game/Blueprints/SettingsWidget.AV_Decrease` (`/Game/Blueprints/MagePawn_BP.WidgetRef` _asmage_pawn_bp))))

(event `self.AV_dec.OnComponentEndOverlap`
  (params (OverlappedComponent :type "PrimitiveComponent Object Reference") (OtherActor :type "Actor Object Reference") (OtherComp :type "PrimitiveComponent Object Reference") (OtherBodyIndex :type Integer))
  (cast `/Game/Blueprints/MagePawn_BP` OtherActor)
  (set `self.OverlapEnded` true))

(event `self.AV_inc.OnComponentBeginOverlap`
  (params (OverlappedComponent :type "PrimitiveComponent Object Reference") (OtherActor :type "Actor Object Reference") (OtherComp :type "PrimitiveComponent Object Reference") (OtherBodyIndex :type Integer) (bFromSweep :type Boolean) (SweepResult :type "HitResult Structure (by ref)"))
  (bind _asmage_pawn_bp (cast `/Game/Blueprints/MagePawn_BP` OtherActor))
  (set `self.OverlapEnded` false)
  (`KismetSystemLibrary.Delay` 1.0)
  (if (not (`self.OverlapEnded`))
    (`/Game/Blueprints/SettingsWidget.AV_Increase` (`/Game/Blueprints/MagePawn_BP.WidgetRef` _asmage_pawn_bp))))

(event `self.AV_inc.OnComponentEndOverlap`
  (params (OverlappedComponent :type "PrimitiveComponent Object Reference") (OtherActor :type "Actor Object Reference") (OtherComp :type "PrimitiveComponent Object Reference") (OtherBodyIndex :type Integer))
  (cast `/Game/Blueprints/MagePawn_BP` OtherActor)
  (set `self.OverlapEnded` true))

(event `self.EV_dec.OnComponentBeginOverlap`
  (params (OverlappedComponent :type "PrimitiveComponent Object Reference") (OtherActor :type "Actor Object Reference") (OtherComp :type "PrimitiveComponent Object Reference") (OtherBodyIndex :type Integer) (bFromSweep :type Boolean) (SweepResult :type "HitResult Structure (by ref)"))
  (bind _asmage_pawn_bp (cast `/Game/Blueprints/MagePawn_BP` OtherActor))
  (set `self.OverlapEnded` false)
  (`KismetSystemLibrary.Delay` 1.0)
  (if (not (`self.OverlapEnded`))
    (`/Game/Blueprints/SettingsWidget.EV_Decrease` (`/Game/Blueprints/MagePawn_BP.WidgetRef` _asmage_pawn_bp))))

(event `self.EV_dec.OnComponentEndOverlap`
  (params (OverlappedComponent :type "PrimitiveComponent Object Reference") (OtherActor :type "Actor Object Reference") (OtherComp :type "PrimitiveComponent Object Reference") (OtherBodyIndex :type Integer))
  (cast `/Game/Blueprints/MagePawn_BP` OtherActor)
  (set `self.OverlapEnded` true))

(event `self.EV_inc.OnComponentBeginOverlap`
  (params (OverlappedComponent :type "PrimitiveComponent Object Reference") (OtherActor :type "Actor Object Reference") (OtherComp :type "PrimitiveComponent Object Reference") (OtherBodyIndex :type Integer) (bFromSweep :type Boolean) (SweepResult :type "HitResult Structure (by ref)"))
  (bind _asmage_pawn_bp (cast `/Game/Blueprints/MagePawn_BP` OtherActor))
  (set `self.OverlapEnded` false)
  (`KismetSystemLibrary.Delay` 1.0)
  (if (not (`self.OverlapEnded`))
    (`/Game/Blueprints/SettingsWidget.EV_Increase` (`/Game/Blueprints/MagePawn_BP.WidgetRef` _asmage_pawn_bp))))

(event `self.EV_inc.OnComponentEndOverlap`
  (params (OverlappedComponent :type "PrimitiveComponent Object Reference") (OtherActor :type "Actor Object Reference") (OtherComp :type "PrimitiveComponent Object Reference") (OtherBodyIndex :type Integer))
  (cast `/Game/Blueprints/MagePawn_BP` OtherActor)
  (set `self.OverlapEnded` true))

(event `self.Back.OnComponentBeginOverlap`
  (params (OverlappedComponent :type "PrimitiveComponent Object Reference") (OtherActor :type "Actor Object Reference") (OtherComp :type "PrimitiveComponent Object Reference") (OtherBodyIndex :type Integer) (bFromSweep :type Boolean) (SweepResult :type "HitResult Structure (by ref)"))
  (bind _asmage_pawn_bp (cast `/Game/Blueprints/MagePawn_BP` OtherActor))
  (set `self.OverlapEnded` false)
  (`KismetSystemLibrary.Delay` 1.0)
  (if (not (`self.OverlapEnded`))
    (`/Game/Blueprints/SettingsWidget.SetBack` (`/Game/Blueprints/MagePawn_BP.WidgetRef` _asmage_pawn_bp))
    (`SceneComponent.SetVisibility` (`self.Widget`) false false)
    (for _array_element (`SceneComponent.GetChildrenComponents` (`self.DefaultSceneRoot`) true)
      (bind _asprimitive_component (cast `PrimitiveComponent` _array_element))
      (set `PrimitiveComponent.bGenerateOverlapEvents` false _asprimitive_component))
    (bind _outactors (`GameplayStatics.GetAllActorsWithTag` "WRE"))
    (`SceneComponent.SetVisibility` (`Actor.RootComponent` (`|GetArrayItem` _outactors)) true false)))

(event `self.Back.OnComponentEndOverlap`
  (params (OverlappedComponent :type "PrimitiveComponent Object Reference") (OtherActor :type "Actor Object Reference") (OtherComp :type "PrimitiveComponent Object Reference") (OtherBodyIndex :type Integer))
  (cast `/Game/Blueprints/MagePawn_BP` OtherActor)
  (set `self.OverlapEnded` true))

(event `self.Apply.OnComponentBeginOverlap`
  (params (OverlappedComponent :type "PrimitiveComponent Object Reference") (OtherActor :type "Actor Object Reference") (OtherComp :type "PrimitiveComponent Object Reference") (OtherBodyIndex :type Integer) (bFromSweep :type Boolean) (SweepResult :type "HitResult Structure (by ref)"))
  (bind _asmage_pawn_bp (cast `/Game/Blueprints/MagePawn_BP` OtherActor))
  (set `self.OverlapEnded` false)
  (`KismetSystemLibrary.Delay` 1.0)
  (if (not (`self.OverlapEnded`))
    (`/Game/Blueprints/SettingsWidget.Apply` (`/Game/Blueprints/MagePawn_BP.WidgetRef` _asmage_pawn_bp))
    (`SceneComponent.SetVisibility` (`self.Widget`) false false)
    (for _array_element (`SceneComponent.GetChildrenComponents` (`self.DefaultSceneRoot`) true)
      (bind _asprimitive_component (cast `PrimitiveComponent` _array_element))
      (set `PrimitiveComponent.bGenerateOverlapEvents` false _asprimitive_component))
    (bind _outactors (`GameplayStatics.GetAllActorsWithTag` "WRE"))
    (`SceneComponent.SetVisibility` (`Actor.RootComponent` (`|GetArrayItem` _outactors)) true false)))

(event `self.Apply.OnComponentEndOverlap`
  (params (OverlappedComponent :type "PrimitiveComponent Object Reference") (OtherActor :type "Actor Object Reference") (OtherComp :type "PrimitiveComponent Object Reference") (OtherBodyIndex :type Integer))
  (cast `/Game/Blueprints/MagePawn_BP` OtherActor)
  (set `self.OverlapEnded` true))

(fn `test`)

(fn `UserConstructionScript`)