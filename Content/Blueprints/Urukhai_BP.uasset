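; Urukhai enemy that can block the mage's hand strikes and awards score through GameMode_BP when killed.
; BeginPlay starts a muted growl at a random offset.
; A Sword overlap with MagePawn_BP's hand collision plays a block montage and sets Block for its duration, if positive X or Y velocity passes a threshold.
; Death plays a montage, detaches the controller, then destroys the actor after a delay; the SM_Sword overlap only casts.
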(event `self.ReceiveBeginPlay`
  (bind _growl (`self.Growl`))
  (`AudioComponent.SetVolumeMultiplier` _growl 0.0)
  (`AudioComponent.Play` _growl (`KismetMathLibrary.RandomFloatInRange` 2.0 5.0)))

(event `self.OnOrcKilled`
  (set `self.Died` true)
  (`AnimInstance.Montage_Play` (`SkeletalMeshComponent.GetAnimInstance` (`self.Mesh`)) "/Game/Blueprints/OrcAnimation/DyingMontage.DyingMontage" 1.0 "Duration" 0.0 true)
  (`self.DetachFromControllerPendingDestroy` self)
  (`KismetSystemLibrary.Delay` 2.0)
  (`self.K2_DestroyActor` self)
  (bind _asgame_mode_bp (cast `/Game/Blueprints/GameMode_BP` (`GameplayStatics.GetGameMode`)))
  (`/Game/Blueprints/GameMode_BP.AddScore` _asgame_mode_bp))

(event `self.SM_Sword.OnComponentBeginOverlap`
  (params (OverlappedComponent :type "PrimitiveComponent Object Reference") (OtherActor :type "Actor Object Reference") (OtherComp :type "PrimitiveComponent Object Reference") (OtherBodyIndex :type Integer) (bFromSweep :type Boolean) (SweepResult :type "HitResult Structure (by ref)"))
  (cast `/Game/Blueprints/MagePawn_BP` OtherActor))

(event `self.Sword.OnComponentBeginOverlap`
  (params (OverlappedComponent :type "PrimitiveComponent Object Reference") (OtherActor :type "Actor Object Reference") (OtherComp :type "PrimitiveComponent Object Reference") (OtherBodyIndex :type Integer) (bFromSweep :type Boolean) (SweepResult :type "HitResult Structure (by ref)"))
  (bind _asmage_pawn_bp (cast `/Game/Blueprints/MagePawn_BP` OtherActor))
  (if (and (not (`self.Died`)) (== OtherComp (`/Game/Blueprints/MagePawn_BP.HandleCollision` _asmage_pawn_bp)) (or (> (.x (`MagePawn.LastVelocity` _asmage_pawn_bp)) 2.0) (>= (.y (`MagePawn.LastVelocity` _asmage_pawn_bp)) 2.0)))
    (set `self.Block` true)
    (bind _returnvalue (`AnimInstance.Montage_Play` (`SkeletalMeshComponent.GetAnimInstance` (`self.Mesh`)) "/Game/Blueprints/OrcAnimation/BlockMontage.BlockMontage" 1.0 "MontageLength" 0.0 true))
    (`KismetSystemLibrary.Delay` _returnvalue)
    (set `self.Block` false)))

(fn `UserConstructionScript`)