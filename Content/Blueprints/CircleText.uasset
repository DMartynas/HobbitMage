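; Actor that displays the player's current circle chance as in-world text.
; On BeginPlay it casts player pawn 0 to MagePawn and stores the reference.
; Every tick it reads that pawn's CircleChance and writes it, with a label, into its TextRender component.
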(event `self.ReceiveBeginPlay`
  (bind _asmage_pawn (cast `MagePawn` (`GameplayStatics.GetPlayerPawn` 0)))
  (set `self.Player` _asmage_pawn))

(event `self.ReceiveTick`
  (params (DeltaSeconds :type "Float (single-precision)"))
  (`TextRenderComponent.K2_SetText` (`self.TextRender`) (`KismetTextLibrary.Conv_StringToText` (`KismetStringLibrary.Concat_StrStr` "Circle chance: " (`KismetStringLibrary.Conv_DoubleToString` (`MagePawn.CircleChance` (`self.Player`)))))))

(fn `UserConstructionScript`)